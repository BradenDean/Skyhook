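; BP_Opossum_Enemy is a 2D sprite enemy that patrols back and forth along the X axis and can be stomped.
; A self-calling UpdateDir event flips direction and rotates the actor each second, while Tick applies movement and sets the flipbook.
; Capsule hits make BP_SpriteCharacter jump without dealing damage; overlapping WeakSpot also makes it jump and destroys the opossum.
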(event `UpdateDir`
  (`KismetSystemLibrary.Delay` 1.0)
  (set `self.Direction` (* (`self.Direction`) -1.0))
  (`self.UpdateDir`)
  (`self.K2_SetActorRotation` (`KismetMathLibrary.ComposeRotators` (`self.K2_GetActorRotation`) (struct :`Yaw` 180.0))))

(event `self.ReceiveBeginPlay`
  (`self.UpdateDir`))

(event `self.ReceiveTick`
  (params (DeltaSeconds :type "Float (single-precision)"))
  (`self.UpdateAnimation`)
  (`self.AddMovementInput` (1.0 0.0 0.0) (`self.Direction`)))

(event `UpdateAnimation`
  (`PaperFlipbookComponent.SetFlipbook` (`self.Sprite`) "/Game/SunnyLandAssets/sprites/opossum/opossum_flipbook.opossum_flipbook"))

(event `self.CapsuleComponent.OnComponentHit`
  (params (HitComponent :type "PrimitiveComponent Object Reference") (OtherActor :type "Actor Object Reference") (OtherComp :type "PrimitiveComponent Object Reference") (NormalImpulse :type "Vector Structure") (Hit :type "HitResult Structure (by ref)"))
  (bind _asbp_sprite_character (cast `/Game/Blueprints/BP_SpriteCharacter` OtherActor))
  (`self.Jump` _asbp_sprite_character))

(event `self.weakSpot.OnComponentBeginOverlap`
  (params (OverlappedComponent :type "PrimitiveComponent Object Reference") (OtherActor :type "Actor Object Reference") (OtherComp :type "PrimitiveComponent Object Reference") (OtherBodyIndex :type Integer) (bFromSweep :type Boolean) (SweepResult :type "HitResult Structure (by ref)"))
  (bind _asbp_sprite_character (cast `/Game/Blueprints/BP_SpriteCharacter` OtherActor))
  (`self.Jump` _asbp_sprite_character)
  (`self.K2_DestroyActor`))

(fn `UserConstructionScript`)