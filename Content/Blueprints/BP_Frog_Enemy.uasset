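; Frog enemy that hops in place on a repeating timer and can be killed by the player's BP_SpriteCharacter.
; StartJumping calls Jump, then re-invokes itself after a two-second delay, starting from BeginPlay.
; Capsule hits teleport the player to its SpawnLocation, while a WeakSpot overlap destroys the frog, each playing a sound.
; UpdateAnimation runs every Tick but is empty.
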(event `self.ReceiveBeginPlay`
  (`self.StartJumping`))

(event `self.ReceiveTick`
  (params (DeltaSeconds :type "Float (single-precision)"))
  (`self.UpdateAnimation`))

(event `StartJumping`
  (`self.Jump`)
  (`KismetSystemLibrary.Delay` 2.0)
  (`self.StartJumping`))

(event `UpdateAnimation`)

(event `self.CapsuleComponent.OnComponentHit`
  (params (HitComponent :type "PrimitiveComponent Object Reference") (OtherActor :type "Actor Object Reference") (OtherComp :type "PrimitiveComponent Object Reference") (NormalImpulse :type "Vector Structure") (Hit :type "HitResult Structure (by ref)"))
  (bind _asbp_sprite_character (cast `/Game/Blueprints/BP_SpriteCharacter` OtherActor))
  (`SceneComponent.K2_SetWorldLocation` (`Actor.RootComponent` _asbp_sprite_character) (`/Game/Blueprints/BP_SpriteCharacter.spawnLocation` _asbp_sprite_character) false false)
  (`GameplayStatics.SpawnSoundAtLocation` "/Engine/VREditor/Sounds/UI/Leave_Simulate.Leave_Simulate" (`SceneComponent.K2_GetComponentLocation` (`self.CapsuleComponent`)) (struct) 1.0 1.0 0.0 null null))

(event `self.weakSpot.OnComponentBeginOverlap`
  (params (OverlappedComponent :type "PrimitiveComponent Object Reference") (OtherActor :type "Actor Object Reference") (OtherComp :type "PrimitiveComponent Object Reference") (OtherBodyIndex :type Integer) (bFromSweep :type Boolean) (SweepResult :type "HitResult Structure (by ref)"))
  (cast `/Game/Blueprints/BP_SpriteCharacter` OtherActor)
  (`GameplayStatics.SpawnSoundAtLocation` "/Engine/VREditor/Sounds/VR_click3.VR_click3" (`SceneComponent.K2_GetComponentLocation` (`self.CapsuleComponent`)) (struct) 1.0 1.0 0.0 null null)
  (`self.K2_DestroyActor`))

(fn `UserConstructionScript`)